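; Game mode for an eye-tracking app that sets up the scene and manages experiment recording.
; BeginPlay applies saved tracker, glasses and WAMP settings, spawns the ground plane, and adds outline post-process and camera UI; EndPlay saves settings.
; Global event system delegates display error messages and handle experiment start/stop, with flags deferring record widget clicks to Tick.
; It also lends out preloaded MediaTextures from a pool tracked by in-use flags.
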(event `self.ReceiveBeginPlay`
  (bind _returnvalue (`SynOpticonState.GetGlobalEventSystem`))
  ;[1 1 1] Begin Play
  (`self.PrepareMediaTexturePool`)
  (bind _returnvalue_2 (`KismetMaterialLibrary.CreateDynamicMaterialInstance` "/Game/Materials/GazeActorMaterials/PPOutlineInstance.PPOutlineInstance" "PPOutlineInstance"))
  (`PostProcessComponent.AddOrUpdateBlendable` (`self.PostProcess`) _returnvalue_2 1.0)
  (`self.LoadSettings`)
  (`self.SpawnGroundPoint`)
  (`self.SetupGraphicsScalabilitySettings`)
  (`self.CreateSceneCameraWidget`)
  (`|ExecutionSequence`
    (:`then_0`
      (add `GlobalEventSystem.OnErrorMessage` (`SynOpticonState.GetGlobalEventSystem`) (delegate `OnDisplayErrorMessage`)))
    (:`then_1`
      (add `GlobalEventSystem.OnStartExperimentDelegate` _returnvalue (`|CreateDelegate` :!event `StartExperiment`)))
    (:`then_2`
      (add `GlobalEventSystem.OnStopExperimentDelegate` _returnvalue (`|CreateDelegate` :!event `StopExperiment`)))))

(event `OnDisplayErrorMessage`
  (params (_Message :type String))
  ;[1 1 1] Begin Play
  (bind _returnvalue (`|CreateWidget` "/Game/Blueprints/CustomWidgets/PopupWidgets/MessageWidget.MessageWidget_C"))
  (`/Game/Blueprints/CustomWidgets/PopupWidgets/MessageWidget.SetUp` _returnvalue 3.0 (`KismetTextLibrary.Conv_StringToText` _Message))
  (`UserWidget.AddToViewport` _returnvalue 0))

(event `self.ReceiveEndPlay`
  (params (EndPlayReason :type "EEndPlayReason Enum" :default "Destroyed"))
  (bind _returnvalue (`SynOpticonState.GetGlobalEventSystem`))
  ;[1 1 1] End Play
  (`self.SaveSettings`)
  (`|ExecutionSequence`
    (:`then_0`
      (remove `GlobalEventSystem.OnErrorMessage` _returnvalue (delegate `OnDisplayErrorMessage`)))
    (:`then_1`
      (remove `GlobalEventSystem.OnStartExperimentDelegate` _returnvalue (`|CreateDelegate` :!event `StartExperiment`)))
    (:`then_2`
      (remove `GlobalEventSystem.OnStopExperimentDelegate` _returnvalue (`|CreateDelegate` :!event `StopExperiment`)))))

(event `self.ReceiveTick`
  (params (DeltaSeconds :type "Float (single-precision)"))
  (bind _recordwidget (`self.RecordWidget`))
  (`|ExecutionSequence`
    (:`then_0`
      (if (`self.isStartExperiment`)
        (set `self.isStartExperiment` false)
        ;[1 1 1] End Play
        (bind _foundwidgets (`WidgetBlueprintLibrary.GetAllWidgetsOfClass` "/Game/Blueprints/ReplayWidgets/RecordReplayWidget.RecordReplayWidget_C"))
        (if (not (> (`KismetArrayLibrary.Array_Length` _foundwidgets) 0))
          (bind _foundwidgets_2 (`WidgetBlueprintLibrary.GetAllWidgetsOfClass` "/Game/Blueprints/ControlPanelWidgets/ReplayGroupWidget.ReplayGroupWidget_C" false))
          (bind _out (`/Game/Blueprints/ControlPanelWidgets/ReplayGroupWidget.EnableRecordingReplayFunc` (`|GetArrayItem` _foundwidgets_2)))
          (bind _output_get (set `self.RecordWidget` _out)))
        (`/Game/Blueprints/ReplayWidgets/RecordReplayWidget.ClickStartRecording` _output_get)))
    (:`then_1`
      (if (`self.isStopExperiment`)
        (set `self.isStopExperiment` false)
        (`/Engine/EditorBlueprintResources/StandardMacros.IsValid` _recordwidget
          (:`Is Valid`
            (`/Game/Blueprints/ReplayWidgets/RecordReplayWidget.ClickStopRecording` _recordwidget)))))))

(fn `CreateSceneCameraWidget`
  (bind _returnvalue (`|CreateWidget` "/Game/Blueprints/SynOpticonActors/SceneCameraWidget.SceneCameraWidget_C"))
  (`UserWidget.AddToViewport` _returnvalue 0))

(fn `GetMediaTexture`
  (returns (MediaTexture :type "MediaTexture Object Reference"))
  (bind _mediapoolstatus (`self.MediaPoolStatus`))
  (for (_array_element _array_index) _mediapoolstatus
    (if (not _array_element)
      (`KismetArrayLibrary.Array_Set` _mediapoolstatus _array_index true)
      (return (`|GetArrayItem` (`self.MediaTexturePool`) _array_index))))
  (return null))

(fn `LoadSettings`
  (bind _returnvalue (`SettingsJSONExporter.GetSettingsStruct`))
  (`self.SetStateSettings` _returnvalue))

(fn `PrepareMediaTexturePool`
  (bind _returnvalue (`SynOpticonStatics.LoadObjectLibrary` "/Blueprints/MediaTexturePool" "/Script/MediaAssets.MediaTexture"))
  (for _array_element _returnvalue
    (bind _asmedia_texture (cast `MediaTexture` _array_element))
    (`KismetArrayLibrary.Array_Add` (`self.MediaTexturePool`) _asmedia_texture)
    (`KismetArrayLibrary.Array_Add` (`self.MediaPoolStatus`))))

(fn `ReleaseMediaTexture`
  (params (MediaTexture :type "MediaTexture Object Reference"))
  (for (_array_element _array_index) (`self.MediaTexturePool`)
    (if (== _array_element MediaTexture)
      (`KismetArrayLibrary.Array_Set` (`self.MediaPoolStatus`) _array_index))))

(fn `SaveSettings`
  (`SettingsJSONExporter.SaveSettingsStruct` (make `SettingsStruct` (`SynOpticonState.GetTrackerOffset`) (`SynOpticonState.GetGlassesOffset`) (0.0 0.0 0.0) 100.0 0.1 (`SynOpticonState.IsHorizontalCoordinateSystem`) 0.0 (`SynOpticonState.GetScreenSaveRateFPS`) (not (`SynOpticonState.IsScreenSaveRatePerSeconds`)) (`SynOpticonState.GetWAMPRouterAdress`) (`SynOpticonState.GetWAMPRealm`))))

(fn `SetStateSettings`
  (params (Settings :type "SettingsStruct Structure"))
  (`|ExecutionSequence`
    (:`then_0`
      (`SynOpticonState.SetTrackerOffset` Settings_MotiveOffset))
    (:`then_1`
      (`SynOpticonState.SetGlassesOffset` Settings_ETOffset))
    (:`then_2`
      (`SynOpticonState.SetHorizontalCoordinateSystem` Settings_IsHorizontalCoordinateSystem))
    (:`then_3`
      (`SynOpticonState.SetScreenSaveRate` Settings_SaveScreenRate Settings_bSaveRatePerMinute))
    (:`then_4`
      (`SynOpticonState.SetWAMPRouterAdress` Settings_CrossbarAdress))
    (:`then_5`
      (`SynOpticonState.SetWAMPRealm` Settings_CrossbarRealm))))

(fn `SetupGraphicsScalabilitySettings`
  (bind _returnvalue (`GameUserSettings.GetGameUserSettings`))
  (`GameUserSettings.LoadSettings` _returnvalue false)
  (`KismetSystemLibrary.ExecuteConsoleCommand` "r.streaming.poolsize 1024" null)
  (`GameUserSettings.ApplySettings` _returnvalue true))

(fn `SpawnGroundPoint`
  (bind _returnvalue (`|SpawnActorFromClass` "/Game/Blueprints/GroundPointBP.GroundPointBP_C" (`KismetMathLibrary.MakeTransform` (`SynOpticonState.GetGroundPointLocation`) (`SynOpticonState.GetGroundPointRotation`)) "Undefined" "OverrideRootScale" null null))
  (bind _output_get (set `self.GroundPlane` _returnvalue))
  (`/Game/Blueprints/GroundPointBP.SetCollisionBoxOrientation` _output_get (`SynOpticonState.IsHorizontalCoordinateSystem`)))

(fn `StartExperiment`
  (if (not (or (`SynOpticonState.IsReplaying`) (`SynOpticonState.IsRecording`)))
    (set `self.isStartExperiment` true)))

(fn `StopExperiment`
  (if (`SynOpticonState.IsRecording`)
    (set `self.isStopExperiment` true)))

(fn `UserConstructionScript`)