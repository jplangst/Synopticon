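; An actor that shows frames from an RTSP client on its Display component.
; On BeginPlay it creates a dynamic material instance, applies it to the first material slot of Display, and binds to the client's OnFrameReceived event.
; Each received frame's texture is written to the material's Texture parameter, so updates are event-driven without Tick.
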(event `self.ReceiveBeginPlay`
  (`self.Setup Display`)
  (add `RtspClientComponent.OnFrameReceived` (`self.RtspClient`) (delegate `OnFrameReceived_Event`)))

(event `OnFrameReceived_Event`
  (params (Texture :type "Texture2D Object Reference"))
  (`MaterialInstanceDynamic.SetTextureParameterValue` (`self.DisplayMaterial`) "Texture" Texture))

(fn `Setup Display`
  (bind _returnvalue (`KismetMaterialLibrary.CreateDynamicMaterialInstance` null))
  (bind _output_get (set `self.DisplayMaterial` _returnvalue))
  (`PrimitiveComponent.SetMaterial` (`self.Display`) 0 _output_get))

(fn `UserConstructionScript`)