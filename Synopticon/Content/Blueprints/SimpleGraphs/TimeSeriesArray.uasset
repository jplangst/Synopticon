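; Time-series sample buffer for simple graphs, storing 2D points with X as time and Y as value.
; AddValue appends a point, prunes leading samples over one time unit older than it, and tracks the first remaining time.
; GetMinMaxValues scans for axis bounds, with minimum X seeded at zero.
; InitArray stores a time range, but pruning uses a hardcoded window instead.
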(fn `AddValue`
  (params (Value :type "Vector2D Structure"))
  (locals (RemoveAllIncludingIndex :type Integer) (ItemsToRemove :type "Array of Vector2D Structure"))
  (set `local.RemoveAllIncludingIndex` -1)
  (`KismetArrayLibrary.Array_Add` (`self.Container`) Value)
  (for (_array_element _array_index) (`self.Container`)
    (bind _x (`KismetMathLibrary.BreakVector2D` _array_element))
    (if (> (- (`KismetMathLibrary.BreakVector2D` (`local.Value`)) _x) 1.0)
      (set `local.RemoveAllIncludingIndex` _array_index)
      (`KismetArrayLibrary.Array_Add` (`local.ItemsToRemove`) _array_element)
      (else
        (set `self.FirstTimeValue` _x)
        (break))))
  (if (!= (`local.RemoveAllIncludingIndex`) -1)
    (for _array_element_2 (`local.ItemsToRemove`)
      (`KismetArrayLibrary.Array_RemoveItem` (`self.Container`) _array_element_2))))

(fn `ClearArray`
  (`KismetArrayLibrary.Array_Clear` (`self.Container`)))

(fn `GetArray`
  (returns (Array :type "Array of Vector2D Structure"))
  (return (`self.Container`)))

(fn `GetFirstTimeValue`
  (returns (FirstTimeValue :type "Float (double-precision)"))
  (return (`self.FirstTimeValue`)))

(fn `GetMinMaxValues`
  (returns (MinMaxX :type "Vector2D Structure") (MinMaxY :type "Vector2D Structure"))
  (locals (MinY :type "Float (double-precision)") (MaxY :type "Float (double-precision)") (MinX :type "Float (double-precision)") (MaxX :type "Float (double-precision)"))
  (for (_array_element _array_index) (`self.Container`)
    (if (== _array_index 0)
      (bind (_x _y) (`KismetMathLibrary.BreakVector2D` _array_element))
      (bind _output_get (set `local.MinY` _y))
      (set `local.MaxY` _output_get)
      (set `local.MinX` 0.0)
      (set `local.MaxX` _x)
      (else
        (`|ExecutionSequence`
          (:`then_0`
            (if (< _y (`local.MinY`))
              (set `local.MinY` _y)))
          (:`then_1`
            (if (> _y (`local.MaxY`))
              (set `local.MaxY` _y)))
          (:`then_2`
            (if (< _x (`local.MinX`))
              (set `local.MinX` _x)))
          (:`then_3`
            (if (> _x (`local.MaxX`))
              (set `local.MaxX` _x)))))))
  (return (`KismetMathLibrary.MakeVector2D` (`local.MinX`) (`local.MaxX`)) (`KismetMathLibrary.MakeVector2D` (`local.MinY`) (`local.MaxY`))))

(fn `InitArray`
  (params (TimeRangeFromLastSample :type "Float (double-precision)"))
  (set `self.TimeRangeFromLastSample` TimeRangeFromLastSample)
  (`KismetArrayLibrary.Array_Clear` (`self.Container`)))