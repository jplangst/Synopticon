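; Fixed-size circular buffer of numeric samples in the SimpleGraphs folder, with min and max queries over its contents.
; InitArray zero-fills the container, so it is always full, and each AddValue advances End and Begin with modulo wrap to overwrite the oldest slot.
; GetArray unrolls the ring from Begin into linear order, while GetCircularArray exposes the raw container, size and start index.
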(fn `AddValue`
  (params (Value :type "Float (double-precision)"))
  (`|ExecutionSequence`
    (:`then_0`
      (bind _result (`/Engine/EditorBlueprintResources/StandardMacros.IncrementInt` (`self.End`))
        (:`  `
          (set `self.End` (mod _result (`self.Size`))))))
    (:`then_1`
      (`KismetArrayLibrary.Array_Set` (`self.Container`) (`self.End`) Value))
    (:`then_2`
      (bind _result_2 (`/Engine/EditorBlueprintResources/StandardMacros.IncrementInt` (`self.Begin`))
        (:`  `
          (set `self.Begin` (mod _result_2 (`self.Size`))))))))

(fn `GetArray`
  (returns (Array :type "Array of Float (double-precision)"))
  (locals (LinearArray :type "Array of Float (double-precision)"))
  (for _index (range (`self.Size`))
    (`KismetArrayLibrary.Array_Add` (`local.LinearArray`) (`|GetArrayItem` (`self.Container`) (mod (+ _index (`self.Begin`)) (`self.Size`)))))
  (return (`local.LinearArray`)))

(fn `GetCircularArray`
  (returns (CircularArray :type "Array of Float (double-precision)") (Size :type Integer) (Begin :type Integer))
  (return (`self.Container`) (`self.Size`) (`self.Begin`)))

(fn `GetMinMaxValues`
  (returns (MinMax :type "Vector2D Structure"))
  (locals (MinY :type "Float (double-precision)") (MaxY :type "Float (double-precision)"))
  (for (_array_element _array_index) (`self.Container`)
    (if (== _array_index 0)
      (bind _output_get (set `local.MinY` _array_element))
      (set `local.MaxY` _output_get)
      (else
        (`|ExecutionSequence`
          (:`then_0`
            (if (< _array_element (`local.MinY`))
              (set `local.MinY` _array_element)))
          (:`then_1`
            (if (> _array_element (`local.MaxY`))
              (set `local.MaxY` _array_element)))))))
  (return (`KismetMathLibrary.MakeVector2D` (`local.MinY`) (`local.MaxY`))))

(fn `InitArray`
  (params (ArraySize :type Integer))
  (bind _container (`self.Container`))
  (set `self.Size` ArraySize)
  (set `self.Begin` 0)
  (set `self.End` -1)
  (`KismetArrayLibrary.Array_Clear` _container)
  (for _ (range (`self.Size`))
    (`KismetArrayLibrary.Array_Add` _container)))