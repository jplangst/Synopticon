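; Player controller for an eye-tracking application that handles input, creates the control panel HUD and plays sound effects.
; It traces left clicks to gaze actors, drives right-drag camera look and Shift-wheel pawn speed, and toggles debug options.
; Key releases route to modelling-menu hotkeys when that menu is open, otherwise to hotbar widgets.
; Calibration functions spawn colour-coded markers at picked points and step through them via EyeTrackingGameMode.
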(event `Key|LeftMouseButton`
  (params (Key :type "Key Structure"))
  (bind (_worldlocation _worlddirection) (`self.DeprojectMousePositionToWorld`))
  ;[1 1 1] Mouse clicked
  (:`Pressed`
    (if (`|EnumInequality` (`self.MenuContext`) "DialogContext")
      (bind _outhit (`KismetSystemLibrary.LineTraceSingle` _worldlocation (+ _worldlocation (* _worlddirection 1000.0)) "TraceTypeQuery5"))
      (bind (_bblockinghit _binitialoverlap _time _distance _location _impactpoint _normal _impactnormal _physmat _hitactor _hitcomponent _hitbonename _bonename _hititem _elementindex _faceindex) (`GameplayStatics.BreakHitResult` _outhit))
      (bind _asgaze_actor_blueprint (cast `/Game/Blueprints/GazeObjects/GazeActorBlueprint` _hitactor))
      (`/Game/Blueprints/GazeObjects/GazeActorBlueprint.OnActorClicked` _asgaze_actor_blueprint _location _faceindex))))

(event `Key|AnyKey` :consume false
  (params (Key :type "Key Structure"))
  ;[1 1 1] Handle the hotkeys of all the sub menus and when there should be no hotkeys
  (:`Released`
    (if (`KismetInputLibrary.Key_IsKeyboardKey` Key)
      (bind _foundwidgets (`WidgetBlueprintLibrary.GetAllWidgetsOfClass` "/Game/Blueprints/PositionModelling/PositionModellingMenu.PositionModellingMenu_C"))
      (if (> (`KismetArrayLibrary.Array_Length` _foundwidgets) 0)
        (`self.HandleModellingHotkeys` Key (`|GetArrayItem` _foundwidgets))
        (else
          (`self.HandleHotkeyInput` Key))))))

(event `self.ReceiveBeginPlay`
  (bind _returnvalue (`SynOpticonState.GetGlobalEventSystem`))
  ;[1 1 1] Begin and End Play
  (add `GlobalEventSystem.OnEventEnterMenuContext` _returnvalue (delegate `ContextChange`))
  (add `GlobalEventSystem.OnPlaySoundEffect` _returnvalue (`|CreateDelegate` :!event `PlaySoundEffect`))
  (set `self.message` (`self.MAIN`))
  (`/Engine/EditorBlueprintResources/StandardMacros.NegateFloat` (`self.GetDeprecatedInputPitchScale`)
    (:`  `
      (bind _returnvalue_2 (`|CreateWidget` "/Game/Blueprints/ControlPanelWidgets/ControlPanelBP.ControlPanelBP_C"))
      (`UserWidget.AddToViewport` _returnvalue_2 0)
      (`self.ClientSetHUD` "/Script/Engine.HUD"))))

(event `ContextChange`
  (params (MenuContext :type "UIContextEnum Enum" :default "DialogContext"))
  ;[1 1 1] Begin and End Play
  (set `self.MenuContext` MenuContext))

(event `self.ReceiveEndPlay`
  (params (EndPlayReason :type "EEndPlayReason Enum" :default "Destroyed"))
  (bind _returnvalue (`SynOpticonState.GetGlobalEventSystem`))
  ;[1 1 1] Begin and End Play
  (remove `GlobalEventSystem.OnEventEnterMenuContext` _returnvalue (delegate `ContextChange`))
  (remove `GlobalEventSystem.OnPlaySoundEffect` _returnvalue (`|CreateDelegate` :!event `PlaySoundEffect`)))

(event `Key|MouseScrollDown`
  (params (Key :type "Key Structure"))
  ;[1 1 1] Change Movement Speed
  (:`Pressed`
    (if (`self.ShiftActive`)
      (bind _assyn_opticon_pawn (cast `SynOpticonPawn` (`self.K2_GetPawn`)))
      (`SynOpticonPawn.AddMovementRate` _assyn_opticon_pawn -0.02))))

(event `Key|MouseScrollUp`
  (params (Key :type "Key Structure"))
  ;[1 1 1] Change Movement Speed
  (:`Pressed`
    (if (`self.ShiftActive`)
      (bind _assyn_opticon_pawn (cast `SynOpticonPawn` (`self.K2_GetPawn`)))
      (`SynOpticonPawn.AddMovementRate` _assyn_opticon_pawn 0.02))))

(event `Key|LeftShift`
  (params (Key :type "Key Structure"))
  ;[1 1 1] Change Movement Speed
  (:`Pressed`
    (set `self.ShiftActive` true))
  (:`Released`
    (set `self.ShiftActive` false)))

(event `InputAction|SelectCalPoints`
  (params (Key :type "Key Structure"))
  (:`Released`
    (if (`self.isChoosingCalPoint`)
      (`self.SelectingCalPoints`))))

(event `InputAxisKey|MouseX`
  (params (AxisValue :type "Float (single-precision)"))
  ;[1 1 1] New way to control camera
  (bind _assyn_opticon_pawn (cast `SynOpticonPawn` (`GameplayStatics.GetPlayerPawn` 0)))
  (if (and (`self.IsTurning`) (`SynOpticonPawn.IsMovementAllowed` _assyn_opticon_pawn))
    (`self.AddYawInput` AxisValue)))

(event `InputAxisKey|MouseY`
  (params (AxisValue :type "Float (single-precision)"))
  ;[1 1 1] New way to control camera
  (bind _assyn_opticon_pawn (cast `SynOpticonPawn` (`GameplayStatics.GetPlayerPawn` 0)))
  (if (and (`self.IsTurning`) (`SynOpticonPawn.IsMovementAllowed` _assyn_opticon_pawn))
    (`self.AddPitchInput` AxisValue)))

(event `Key|RightMouseButton`
  (params (Key :type "Key Structure"))
  ;[1 1 1] New way to control camera
  (:`Pressed`
    (set `self.IsTurning` true))
  (:`Released`
    (set `self.IsTurning` false)))

(event `InputAction|StatUnit`
  (params (Key :type "Key Structure"))
  ;[1 1 1] Debug
  ;;[1 1 1] Show FPS
  (:`Pressed`
    (`KismetSystemLibrary.ExecuteConsoleCommand` "stat Unit" null)))

(event `InputAction|StartSampling`
  (params (Key :type "Key Structure"))
  ;[1 1 1] Debug
)

(event `InputAction|FramePerSecond`
  (params (Key :type "Key Structure"))
  ;[1 1 1] Debug
  ;;[1 1 1] Show FPS
  (:`Pressed`
    (`KismetSystemLibrary.ExecuteConsoleCommand` "stat FPS" null)))

(event `InputAction|StopSampling`
  (params (Key :type "Key Structure"))
  ;[1 1 1] Debug
)

(event `InputAction|StatGame`
  (params (Key :type "Key Structure"))
  ;[1 1 1] Debug
)

(event `InputAction|MemReport`
  (params (Key :type "Key Structure"))
  ;[1 1 1] Debug
  ;;[1 1 1] Alt-M
)

(event `InputAction|DumpFrame`
  (params (Key :type "Key Structure"))
  ;[1 1 1] Debug
)

(event `InputAction|ApplyOffset`
  (params (Key :type "Key Structure"))
  ;[1 1 1] Debug
  (:`Released`
    (bind _returnvalue (`SynOpticonState.ShouldApplyOffset`))
    (`SynOpticonState.ApplyOffset` (not _returnvalue))))

(event `InputAction|ShowDebugLines`
  (params (Key :type "Key Structure"))
  ;[1 1 1] Debug
  (:`Released`
    (bind _returnvalue (`SynOpticonState.IsShowingDebugLines`))
    (`SynOpticonState.ShowDebugLines` (not _returnvalue))))

(fn `ActivateCalPointSelection`
  (bind _calibrationpointactors (`self.CalibrationPointActors`))
  (if (`self.isChoosingCalPoint`)
    (set `self.isChoosingCalPoint` false)
    (else
      (set `self.CalibrationIndex` 0)
      (set `self.isChoosingCalPoint` true)
      ;[1 1 1] Remove existing calibration points
      (for _array_element _calibrationpointactors
        (`self.K2_DestroyActor` _array_element))
      (`KismetArrayLibrary.Array_Clear` _calibrationpointactors)
      (bind _aseye_tracking_game_mode (cast `EyeTrackingGameMode` (`GameplayStatics.GetGameMode`))
        (:`then`
          (`EyeTrackingGameMode.ClearCalibrationPoints` _aseye_tracking_game_mode)
          ;[1 1 1] Prepare for calibration point selection
          (set `self.CurrentMouseCursor` "Hand")
          (set `self.message` (`KismetStringLibrary.Concat_StrStr` "Calibration Mode: click on screen to choose " " calibration points")))
        (:`CastFailed`
          _))))
  (return))

(fn `ChangeTrackingSound`
  (params (Tracking :type Boolean))
  (bind _tooltrackingsound (`self.ToolTrackingSound`))
  (if Tracking
    (`AudioComponent.SetIntParameter` _tooltrackingsound "Tracking" 0)
    (else
      (`AudioComponent.SetIntParameter` _tooltrackingsound "Tracking" 1))))

(fn `HandleHotkeyInput`
  (params (Key :type "Key Structure"))
  (`|ExecutionSequence`
    (:`then_0`
      (if (`self.isKeyBinding`)
        (if (== (`local.Key`) "Escape")
          ;[1 1 1] Exit application
          (bind _foundwidgets (`WidgetBlueprintLibrary.GetAllWidgetsWithInterface` "/Game/Blueprints/ControlPanelWidgets/HotbarGroupWidgetInterface.HotbarGroupWidgetInterface_C"))
          (for _array_element _foundwidgets
            (if (`|EnumInequality` (`Widget.GetVisibility` _array_element) "Hidden")
              (set `self.isAbleToClose` false)
              (break)))
          (if (`self.isAbleToClose`)
            (`KismetSystemLibrary.ExecuteConsoleCommand` "EXIT" null)
            (else
              (set `self.isAbleToClose` true))))))
    (:`then_1`
      (if (not (`SynOpticonState.GetScreenLabeling`))
        ;[1 1 1] Check the pressed key against the hotbar buttons registered hotkey
        (bind _foundwidgets_2 (`WidgetBlueprintLibrary.GetAllWidgetsOfClass` "/Game/Blueprints/ControlPanelWidgets/HotbarButtonWidget.HotbarButtonWidget_C" false))
        (for _array_element_2 _foundwidgets_2
          (if (`Widget.GetIsEnabled` _array_element_2)
            (bind _hotkey (`/Game/Blueprints/ControlPanelWidgets/HotbarButtonWidget.GetHotkey` _array_element_2))
            (if (== _hotkey (`local.Key`))
              (`/Game/Blueprints/ControlPanelWidgets/HotbarButtonWidget.ClickButton` _array_element_2)
              (break))))))
    (:`then_2`
      ;[1 1 1] Check if the UI_HotbarButtins should be pressed
      (bind _foundwidgets_3 (`WidgetBlueprintLibrary.GetAllWidgetsOfClass` "/Game/Blueprints/UserInterface/UI_HotbarButton.UI_HotbarButton_C" false))
      (for _array_element_3 _foundwidgets_3
        (`/Game/Blueprints/UserInterface/UI_HotbarButton.PressIfHotkey` _array_element_3 (`local.Key`))))))

(fn `HandleModellingHotkeys`
  (params (Key :type "Key Structure" :default "None") (ModellingMenu :type "/Game/Blueprints/PositionModelling/PositionModellingMenu Object Reference"))
  (if (`self.UseModellingHotkeys`)
    (if (== Key "PageDown")
      (`/Game/Blueprints/PositionModelling/PositionModellingMenu.TakeManualMeasurement` ModellingMenu)
      (elif (== Key "PageUp")
        (`/Game/Blueprints/PositionModelling/PositionModellingMenu.RemoveLastMeasurement` ModellingMenu)
        (elif (or (== Key "F5") (== Key "Escape"))
          (`/Game/Blueprints/PositionModelling/PositionModellingMenu.NextGeometryType` ModellingMenu)
          (elif (== Key "Period")
            (`/Game/Blueprints/PositionModelling/PositionModellingMenu.CreateGeometry` ModellingMenu)
            (`/Game/Blueprints/PositionModelling/PositionModellingMenu.ClearLists` ModellingMenu)))))))

(fn `PerformCalibration`
  (locals (numCalPoints :type Integer :default 3))
  (bind _calibrationpointactors (`self.CalibrationPointActors`))
  (bind _calibrationindex (`self.CalibrationIndex`))
  (bind _numcalpoints (`local.numCalPoints`))
  (bind _output_get (set `local.numCalPoints` (`KismetArrayLibrary.Array_Length` (`self.CalibrationPointActors`))))
  (if (> _output_get 0)
    (`MaterialInstanceDynamic.SetVectorParameterValue` (`/Game/Blueprints/CalPointBP.DynamicMaterial` (`|GetArrayItem` (`self.CalibrationPointActors`) (`self.CalibrationIndex`))) "Colour" (`self.CalibratedColor`))
    (`/Engine/EditorBlueprintResources/StandardMacros.IncrementInt` (`self.CalibrationIndex`)
      (:`  `
        (set `self.message` (`KismetStringLibrary.Concat_StrStr` (`self.CALIBRATION`) (`KismetStringLibrary.Conv_IntToString` (+ (`self.CalibrationIndex`) 1))))
        (bind _aseye_tracking_game_mode (cast `EyeTrackingGameMode` (`GameplayStatics.GetGameMode`))
          (:`then`
            (if (<= _calibrationindex _numcalpoints)
              (`EyeTrackingGameMode.CalibrateVectorToPoint` _aseye_tracking_game_mode _calibrationindex)
              (if (== _calibrationindex _numcalpoints)
                (set `self.message` (`self.MAIN`))
                (set `self.CalibrationIndex` 0)
                (for _array_element _calibrationpointactors
                  (`MaterialInstanceDynamic.SetVectorParameterValue` (`/Game/Blueprints/CalPointBP.DynamicMaterial` _array_element) "Colour" (`self.InactiveColor`)))
                (`MaterialInstanceDynamic.SetVectorParameterValue` (`/Game/Blueprints/CalPointBP.DynamicMaterial` (`|GetArrayItem` _calibrationpointactors)) "Colour" (`self.ActiveColor`))
                (else
                  (`MaterialInstanceDynamic.SetVectorParameterValue` (`/Game/Blueprints/CalPointBP.DynamicMaterial` (`|GetArrayItem` (`self.CalibrationPointActors`) _calibrationindex)) "Colour" (`self.ActiveColor`))))))
          (:`CastFailed`
            _)))))
  (return))

(fn `PlaySoundEffect`
  (params (SoundEffect :type "ESoundEffectEnum Enum" :default "SE_PointModelled"))
  (locals (SelectedSound :type "SoundBase Object Reference"))
  (`|ExecutionSequence`
    (:`then_0`
      (switch `ESoundEffectEnum` SoundEffect
        (:`SE_PointModelled`
          (set `local.SelectedSound` "/Game/SoundEffects/SoundEffects/sms-alert-3-daniel_simon.sms-alert-3-daniel_simon"))
        (:`SE_PointRemoved`
          (set `local.SelectedSound` "/Game/SoundEffects/SoundEffects/sms-alert-1-daniel_simon.sms-alert-1-daniel_simon"))))
    (:`then_1`
      (`AudioComponent.SetSound` (`self.SoundEffectsPlayer`) (`local.SelectedSound`))
      (`AudioComponent.Play` (`self.SoundEffectsPlayer`) 0.0))))

(fn `PlayTrackingSound`
  (params (Play :type Boolean))
  (bind _tooltrackingsound (`self.ToolTrackingSound`))
  (if Play
    (`AudioComponent.Play` _tooltrackingsound 0.0)
    (else
      (`AudioComponent.Stop` _tooltrackingsound))))

(fn `PointToText`
  (params (Point :type "Vector Structure"))
  (returns (Text :type String))
  (return (`KismetStringLibrary.Concat_StrStr` (`KismetStringLibrary.Conv_DoubleToString` (.x Point)) ":" (`KismetStringLibrary.Conv_DoubleToString` (.y Point)) ":" (`KismetStringLibrary.Conv_DoubleToString` (.z Point)))))

(fn `SelectingCalPoints`
  (locals (NumCalPointsTMP :type Integer :default 6))
  (bind _calibrationpointactors (`self.CalibrationPointActors`))
  (bind (_bblockinghit _binitialoverlap _time _distance _location _impactpoint _normal _impactnormal _physmat _hitactor) (`GameplayStatics.BreakHitResult` (`self.GetHitResultUnderCursorByChannel` "TraceTypeQuery1")))
  (if (`self.isShowingCP`)
    (bind _aseye_tracking_game_mode (cast `EyeTrackingGameMode` (`GameplayStatics.GetGameMode`))
      (:`then`
        (cast `GazeActor` _hitactor
          (:`then`
            (`EyeTrackingGameMode.AddCalibrationPoint` _aseye_tracking_game_mode _impactpoint)
            (bind _returnvalue (`|SpawnActorFromClass` "/Game/Blueprints/CalPointBP.CalPointBP_C" (`KismetMathLibrary.MakeTransform` _impactpoint (struct) (0.1 0.1 0.1)) "Undefined" "OverrideRootScale" null null))
            (if (== (`KismetArrayLibrary.Array_Length` _calibrationpointactors) 0)
              (`MaterialInstanceDynamic.SetVectorParameterValue` (`/Game/Blueprints/CalPointBP.DynamicMaterial` _returnvalue) "Colour" (`self.ActiveColor`)))
            (`KismetArrayLibrary.Array_Add` _calibrationpointactors _returnvalue)
            (if (>= (`KismetArrayLibrary.Array_Length` (`self.CalibrationPointActors`)) (`local.NumCalPointsTMP`))
              (set `self.CurrentMouseCursor` "Default")))
          (:`CastFailed`
            _)))
      (:`CastFailed`
        _))
    (return)
    (else
      (return))))

(fn `ToggleHideShowCalPoints`
  (set `self.isShowingCP` (not (`self.isShowingCP`)))
  (for _array_element (`self.CalibrationPointActors`)
    (`SceneComponent.ToggleVisibility` (`/Game/Blueprints/CalPointBP.Sphere` _array_element) false))
  (return))

(fn `ToggleOpenSettingPanel`
  (if (not (`self.isShowingSetting`))
    (set `self.isShowingSetting` true)
    (bind _returnvalue (`|CreateWidget` "/Game/Blueprints/ControlPanelWidgets/SettingBP.SettingBP_C"))
    (`UserWidget.AddToViewport` _returnvalue 0)
    (set `self.bShowMouseCursor` true)
    (`WidgetBlueprintLibrary.SetInputMode_UIOnlyEx` self _returnvalue))
  (return))

(fn `UserConstructionScript`)