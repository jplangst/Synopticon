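; GazeDataVisualizerBP configures the materials and parameters of particle systems used to visualize gaze data.
; SetupDynamicMaterial creates and applies a dynamic material from one of two gaze materials, chosen by a Fixation flag.
; It passes system number and total to the particle system, and to the material only for non-fixations.
; UpdateDynamicMaterial refreshes both values on an existing particle system and its dynamic material.
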(event `self.SetupDynamicMaterial`
  (params (ParticleSystem :type "ParticleSystemComponent Object Reference") (Fixation :type Boolean) (MaxSystems :type Integer) (SystemNumber :type Integer))
  (bind _returnvalue (`KismetMathLibrary.Conv_IntToDouble` MaxSystems))
  (bind _returnvalue_2 (`KismetMathLibrary.Conv_IntToDouble` SystemNumber))
  (`|ExecutionSequence`
    (:`then_0`
      (if Fixation
        (bind _returnvalue_3 (`PrimitiveComponent.CreateDynamicMaterialInstance` ParticleSystem 0 "/Game/Materials/GazeParticleMaterial.GazeParticleMaterial"))
        (set `self.DynamicMaterial` _returnvalue_3)
        (else
          (bind _returnvalue_4 (`PrimitiveComponent.CreateDynamicMaterialInstance` ParticleSystem 0 "/Game/Materials/GazeParticleMaterial2.GazeParticleMaterial2"))
          (bind _output_get (set `self.DynamicMaterial` _returnvalue_4))
          (`MaterialInstanceDynamic.SetScalarParameterValue` _output_get "TestMax" _returnvalue)
          (`MaterialInstanceDynamic.SetScalarParameterValue` _output_get "TestNumber" _returnvalue_2))))
    (:`then_1`
      (`PrimitiveComponent.SetMaterial` ParticleSystem 0 (`self.DynamicMaterial`))
      (`ParticleSystemComponent.SetFloatParameter` ParticleSystem "MaxSystems" _returnvalue)
      (`ParticleSystemComponent.SetFloatParameter` ParticleSystem "SystemNumber" _returnvalue_2))))

(event `self.UpdateDynamicMaterial`
  (params (ParticleSystem :type "ParticleSystemComponent Object Reference") (SystemNumber :type Integer) (MaxSystems :type Integer))
  (bind _returnvalue (`KismetMathLibrary.Conv_IntToDouble` MaxSystems))
  (bind _returnvalue_2 (`KismetMathLibrary.Conv_IntToDouble` SystemNumber))
  (`ParticleSystemComponent.SetFloatParameter` ParticleSystem "SystemNumber" _returnvalue_2)
  (`ParticleSystemComponent.SetFloatParameter` ParticleSystem "MaxSystems" _returnvalue)
  (bind _asmaterial_instance_dynamic (cast `MaterialInstanceDynamic` (`PrimitiveComponent.GetMaterial` ParticleSystem 0)))
  (`MaterialInstanceDynamic.SetScalarParameterValue` _asmaterial_instance_dynamic "TestMax" _returnvalue)
  (`MaterialInstanceDynamic.SetScalarParameterValue` _asmaterial_instance_dynamic "TestNumber" _returnvalue_2))