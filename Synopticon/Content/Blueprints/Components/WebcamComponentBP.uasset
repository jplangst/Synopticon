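; WebcamComponentBP is a component that plays a webcam stream in the eye-tracking game.
; On BeginPlay it takes a pooled MediaTexture from the game mode, feeds it into a dynamic material and links it to a new MediaPlayer.
; LoadVideo opens the configured URL only outside replay; UpdateVideoFeed calls it again.
; MediaOpened selects the configured video track and plays after a short delay, and EndPlay closes the player.
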(event `self.ReceiveBeginPlay`
  ;[1 1 1] Get a MediaTexture from the pool
  (bind _aseye_tracking_game_mode_bp (cast `/Game/Blueprints/EyeTrackingGameModeBP` (`GameplayStatics.GetGameMode`)))
  (bind _mediatexture (`/Game/Blueprints/EyeTrackingGameModeBP.GetMediaTexture` _aseye_tracking_game_mode_bp))
  (set `self.VideoTexture` _mediatexture)
  ;[1 1 1] Create and setup the video material and player
  (bind _returnvalue (`KismetMaterialLibrary.CreateDynamicMaterialInstance` "/Game/Materials/VideoComponentPlayerMaterial.VideoComponentPlayerMaterial"))
  (set `self.VideoMaterial` _returnvalue)
  (bind _returnvalue_2 (`|GenericCreateObject` self "/Script/MediaAssets.MediaPlayer"))
  (bind _output_get (set `self.VideoPlayer` _returnvalue_2))
  (`MaterialInstanceDynamic.SetTextureParameterValue` (`self.VideoMaterial`) "MediaTexture" (`self.VideoTexture`))
  (`MediaPlayer.SetVideoTrackFrameRate` _output_get 0 0 10.0)
  (`MediaTexture.SetMediaPlayer` (`self.VideoTexture`) (`self.VideoPlayer`))
  (`self.LoadVideo`))

(event `self.UpdateVideoFeed`
  (`self.LoadVideo`))

(event `self.ReceiveEndPlay`
  (params (EndPlayReason :type "EEndPlayReason Enum" :default "Destroyed"))
  ;[1 1 1] End Play
  (`MediaPlayer.Close` (`self.VideoPlayer`)))

(event `MediaOpened`
  (params (File :type String))
  (bind _videoplayer (`self.VideoPlayer`))
  ;[1 1 1] On Media Opened
  (`MediaPlayer.SelectTrack` _videoplayer "Video" (`.SelectedVideoTrack` (break `VideoComponentStruct` (`self.GetVideoComponentStruct`))))
  (`KismetSystemLibrary.Delay` 0.2)
  (`MediaPlayer.Play` _videoplayer))

(fn `LoadVideo`
  (bind _videoplayer (`self.VideoPlayer`))
  ;[1 1 1] Load the stream url or the recorded file depending on if we are replaying or not
  (if (not (`SynOpticonState.IsReplaying`))
    (`MediaPlayer.OpenUrl` _videoplayer (`.VideoURL` (break `VideoComponentStruct` (`self.GetVideoComponentStruct`))))
    (add `MediaPlayer.OnMediaOpened` _videoplayer (`|CreateDelegate` :!event `MediaOpened`))))