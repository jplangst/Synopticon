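; Manager component that handles creation of SynOpticon and Gaze actors and resolves their name clashes.
; The global create event opens a SynOpticonActorStatistics widget on screen.
; Duplicates are held as structs while DuplicateNamesWidget dispatchers choose replace, skip or rename, recreating actors from that data and refreshing SynActorMenu for some SynOpticon changes.
; Name checks can show warnings; IsGazeActorNameAvaliable returns true when the name is already taken, despite its name.
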(event `self.ReceiveBeginPlay`
  (add `GlobalEventSystem.OnEventCreateSOActor` (`SynOpticonState.GetGlobalEventSystem`) (`|CreateDelegate` :!event `OnEventCreateSOActor`)))

(event `OnEventCreateSOActor`
  (params (ActorID :type Integer))
  (bind _returnvalue (`|CreateWidget` "/Game/Blueprints/SynOpticonActors/SynOpticonActorStatistics.SynOpticonActorStatistics_C" null ActorID))
  (`UserWidget.AddToViewport` _returnvalue 0))

(event `self.ReplaceOrRenameDuplicatedSynOpticonActors`
  (params (items :type "Array of SynOpticonActorStruct Structure (by ref)"))
  (`self.HandleDuplicateSOActors` items))

(event `ReplaceOneDuplicatedSOItem`
  (params (ActorName :type String))
  (bind _duplicatedsoitems (`self.DuplicatedSOItems`))
  (for _array_element _duplicatedsoitems
    (if (`KismetStringLibrary.EqualEqual_StrStr` ActorName (`.ActorName` (break `SynOpticonActorStruct` _array_element)))
      (`self.CreateAndReplaceSynOpticonActorFromStruct` _array_element)
      (`KismetArrayLibrary.Array_RemoveItem` _duplicatedsoitems _array_element)
      (break)))
  (bind _foundwidgets (`WidgetBlueprintLibrary.GetAllWidgetsOfClass` "/Game/Blueprints/SynOpticonActorMenu/SynActorMenu.SynActorMenu_C" :!label _label))
  (for _array_element_2 _foundwidgets
    (`/Game/Blueprints/SynOpticonActorMenu/SynActorMenu.UpdateActorList` _array_element_2)))

(event `ReplaceAllDuplicatedSOItems`
  (bind _duplicatedsoitems (`self.DuplicatedSOItems`))
  (for _array_element _duplicatedsoitems
    (`self.CreateAndReplaceSynOpticonActorFromStruct` _array_element))
  (`KismetArrayLibrary.Array_Clear` _duplicatedsoitems)
  (goto _label))

(event `SkipOneDuplicatedSOItem`
  (params (ActorName :type String))
  (bind _duplicatedsoitems (`self.DuplicatedSOItems`))
  (for _array_element _duplicatedsoitems
    (if (`KismetStringLibrary.EqualEqual_StrStr` ActorName (`.ActorName` (break `SynOpticonActorStruct` _array_element)))
      (`KismetArrayLibrary.Array_RemoveItem` _duplicatedsoitems _array_element)
      (break))))

(event `SkipAllDuplicatedSOItems`
  (`KismetArrayLibrary.Array_Clear` (`self.DuplicatedSOItems`)))

(event `RenameDuplicatedSOItem`
  (params (Old :type "Array of String") (New :type "Array of String"))
  (bind _duplicatedsoitems (`self.DuplicatedSOItems`))
  (for _array_element _duplicatedsoitems
    (bind (_headerversion _actorname _natnetname _eyetrackerstruct _remoteeyetrackerstruct _shimmercomponents _handcomponents _gazelogcomponentdata _lefthandlogcomponentdata _righthandlogcomponentdata _gazedata _hasmyo _markersconfiguration) (break `SynOpticonActorStruct` _array_element))
    (`self.CreateSynOpticonActorFromStruct` (make `SynOpticonActorStruct` _headerversion (`|GetArrayItem` New (`KismetArrayLibrary.Array_Find` Old _actorname)) _natnetname _eyetrackerstruct _remoteeyetrackerstruct _shimmercomponents _handcomponents (struct) (struct) (struct) _gazedata _hasmyo _markersconfiguration)))
  (`KismetArrayLibrary.Array_Clear` _duplicatedsoitems)
  (bind _foundwidgets (`WidgetBlueprintLibrary.GetAllWidgetsOfClass` "/Game/Blueprints/SynOpticonActorMenu/SynActorMenu.SynActorMenu_C"))
  (for _array_element_2 _foundwidgets
    (`/Game/Blueprints/SynOpticonActorMenu/SynActorMenu.UpdateActorList` _array_element_2)))

(event `self.ReplaceOrRenameDuplicatedGazeActors`
  (params (items :type "Array of GazeActorData Structure (by ref)"))
  (bind _gazeactornames (`self.GetAllGazeActorNames`))
  (`KismetArrayLibrary.Array_Clear` (`self.DuplicatedGazeItems`))
  (bind _output_get (set `self.DuplicatedGazeItems` items))
  (bind _returnvalue (`|CreateWidget` "/Game/Blueprints/CustomWidgets/FileManager/DuplicateNamesWidget.DuplicateNamesWidget_C"))
  (for _array_element _output_get
    (`/Game/Blueprints/CustomWidgets/FileManager/DuplicateNamesWidget.SetUp` _returnvalue (`.Name` (break `GazeActorData` _array_element)) _gazeactornames))
  (`UserWidget.AddToViewport` _returnvalue 0)
  (add `/Game/Blueprints/CustomWidgets/FileManager/DuplicateNamesWidget.OnReplaceItemEventDispatcher` _returnvalue (`|CreateDelegate` :!event `ReplaceIOneDuplicatedGazeItem`))
  (add `/Game/Blueprints/CustomWidgets/FileManager/DuplicateNamesWidget.OnReplaceAllItemsEventDispatcher` _returnvalue (`|CreateDelegate` :!event `ReplaceAllDuplicatedGazeItems`))
  (add `/Game/Blueprints/CustomWidgets/FileManager/DuplicateNamesWidget.OnSkipItemEventDispatcher` _returnvalue (`|CreateDelegate` :!event `SkipOneDuplicatedGazeItem`))
  (add `/Game/Blueprints/CustomWidgets/FileManager/DuplicateNamesWidget.OnSkipAllItemsEventDispatcher` _returnvalue (`|CreateDelegate` :!event `SkipAllDuplicatedGazeItems`))
  (add `/Game/Blueprints/CustomWidgets/FileManager/DuplicateNamesWidget.OnRenameEventDispatcher` _returnvalue (`|CreateDelegate` :!event `RenameGazeItems`)))

(event `ReplaceIOneDuplicatedGazeItem`
  (params (ActorName :type String))
  (bind _duplicatedgazeitems (`self.DuplicatedGazeItems`))
  (for _array_element _duplicatedgazeitems
    (if (`KismetStringLibrary.EqualEqual_StrStr` ActorName (`.Name` (break `GazeActorData` _array_element)))
      (`self.CreateAndReplaceRigidBody` _array_element)
      (`KismetArrayLibrary.Array_RemoveItem` _duplicatedgazeitems)
      (break))))

(event `ReplaceAllDuplicatedGazeItems`
  (bind _duplicatedgazeitems (`self.DuplicatedGazeItems`))
  (for _array_element _duplicatedgazeitems
    (`self.CreateAndReplaceRigidBody` _array_element))
  (`KismetArrayLibrary.Array_Clear` _duplicatedgazeitems))

(event `SkipOneDuplicatedGazeItem`
  (params (ActorName :type String))
  (bind _duplicatedgazeitems (`self.DuplicatedGazeItems`))
  (for _array_element _duplicatedgazeitems
    (if (`KismetStringLibrary.EqualEqual_StrStr` ActorName (`.Name` (break `GazeActorData` _array_element)))
      (`KismetArrayLibrary.Array_RemoveItem` _duplicatedgazeitems _array_element)
      (break))))

(event `SkipAllDuplicatedGazeItems`
  (`KismetArrayLibrary.Array_Clear` (`self.DuplicatedGazeItems`)))

(event `RenameGazeItems`
  (params (OldItems :type "Array of String (by ref)") (NewItems :type "Array of String (by ref)"))
  (for _array_element (`self.DuplicatedGazeItems`)
    (bind (_id _version _gazeactortype _isgazeobject _iscollisionobject _name _markers _vertices _uvs _indexes _aois _popupaois _wampscreenid _webbrowserresolution _url _parented _parentscenecompname _movable _natnetname _sizedimensions) (break `GazeActorData` _array_element))
    (`self.CreateRigidBody` (make `GazeActorData` -1 2 "SRT_Screen" false false (`|GetArrayItem` NewItems (`KismetArrayLibrary.Array_Find` OldItems _name)) _markers _vertices _uvs _indexes _aois _popupaois "" (0.0 0.0) _url false "" _movable _natnetname _sizedimensions)))
  (`KismetArrayLibrary.Array_Clear` (`self.DuplicatedGazeItems`)))

(fn `CheckGazeActorNameValidity`
  (params (GazeActorName :type String) (SuppressWarnings :type Boolean))
  (returns (isValid :type Boolean))
  (locals (ActorName :type String) (Supress :type Boolean))
  (set `local.ActorName` GazeActorName)
  (set `local.Supress` SuppressWarnings)
  (for _array_element (`SynOpticonState.GetGazeActorList`)
    (bind _asgaze_actor (cast `GazeActor` _array_element))
    (if (`KismetStringLibrary.EqualEqual_StrStr` (`GazeActor.GetName` _asgaze_actor) (`local.ActorName`))
      (if (`local.Supress`)
        (return false)
        (else
          (bind _returnvalue (`|CreateWidget` "/Game/Blueprints/CustomWidgets/PopupWidgets/ConfirmationOneButtonWidget.ConfirmationOneButtonWidget_C"))
          (`TextBlock.SetText` (`/Game/Blueprints/CustomWidgets/PopupWidgets/ConfirmationOneButtonWidget.msg_box` _returnvalue) (`KismetTextLibrary.Conv_StringToText` (`KismetStringLibrary.Concat_StrStr` (`KismetStringLibrary.Concat_StrStr` "The name \"" (`local.ActorName`)) "\" has been taken. Please choose another one!")))
          (`UserWidget.AddToViewport` _returnvalue 0)
          (return false)))))
  (return true))

(fn `CheckSOActorNameValidity`
  (params (NewName :type String) (OldName :type String) (SupressWarning :type Boolean))
  (returns (isValid :type Boolean))
  (locals (Supress :type Boolean) (NewSOName :type String) (OldSOName :type String))
  (set `local.NewSOName` NewName)
  (set `local.OldSOName` OldName)
  (set `local.Supress` SupressWarning)
  (if (`KismetStringLibrary.EqualEqual_StrStr` (`local.NewSOName`) (`local.OldSOName`))
    (return true)
    (else
      (for _array_element (`SynOpticonState.GetSynOpticonActorList`)
        (bind _assyn_opticon_actor (cast `SynOpticonActor` _array_element))
        (bind _returnvalue (`SynOpticonActor.GetActorName` _assyn_opticon_actor))
        (if (`KismetStringLibrary.EqualEqual_StrStr` _returnvalue (`local.NewSOName`))
          (if (`local.Supress`)
            (return false)
            (else
              (bind _returnvalue_2 (`|CreateWidget` "/Game/Blueprints/CustomWidgets/PopupWidgets/ConfirmationOneButtonWidget.ConfirmationOneButtonWidget_C"))
              (`TextBlock.SetText` (`/Game/Blueprints/CustomWidgets/PopupWidgets/ConfirmationOneButtonWidget.msg_box` _returnvalue_2) (`KismetTextLibrary.Conv_StringToText` (`KismetStringLibrary.Concat_StrStr` "The name \"" (`local.NewSOName`) "\" has been taken. Please choose another one!")))
              (`UserWidget.AddToViewport` _returnvalue_2 0)
              (return false)))))
      (return true))))

(fn `CreateSynOpticonActor`
  (params (ActorData :type "SynOpticonActorStruct Structure"))
  (locals (NewActorData :type "SynOpticonActorStruct Structure") (CurrActorName :type String) (isSOValid :type Boolean :default true))
  (bind _duplicatedsoitems (`self.DuplicatedSOItems`))
  (set `local.NewActorData` ActorData)
  (for _array_element (`SynOpticonState.GetSynOpticonActorList`)
    (bind _assyn_opticon_actor (cast `SynOpticonActor` _array_element))
    (bind _returnvalue (`SynOpticonActor.GetActorName` _assyn_opticon_actor))
    (bind _output_get (set `local.CurrActorName` _returnvalue))
    (if (`KismetStringLibrary.EqualEqual_StrStr` _output_get (`.ActorName` (break `SynOpticonActorStruct` (`local.NewActorData`))))
      (bind _returnvalue_2 (`|CreateWidget` "/Game/Blueprints/CustomWidgets/FileManager/DuplicateNamesWidget.DuplicateNamesWidget_C"))
      (bind _synopticonnames (`self.GetAllSynopticonActorNames`))
      (`/Game/Blueprints/CustomWidgets/FileManager/DuplicateNamesWidget.SetUp` _returnvalue_2 (`local.CurrActorName`) _synopticonnames)
      (add `/Game/Blueprints/CustomWidgets/FileManager/DuplicateNamesWidget.OnRenameEventDispatcher` _returnvalue_2 (`|CreateDelegate` :!event `RenameDuplicatedSOItem`))
      (add `/Game/Blueprints/CustomWidgets/FileManager/DuplicateNamesWidget.OnReplaceItemEventDispatcher` _returnvalue_2 (`|CreateDelegate` :!event `ReplaceOneDuplicatedSOItem`))
      (add `/Game/Blueprints/CustomWidgets/FileManager/DuplicateNamesWidget.OnReplaceAllItemsEventDispatcher` _returnvalue_2 (`|CreateDelegate` :!event `ReplaceAllDuplicatedSOItems`))
      (add `/Game/Blueprints/CustomWidgets/FileManager/DuplicateNamesWidget.OnSkipItemEventDispatcher` _returnvalue_2 (`|CreateDelegate` :!event `SkipOneDuplicatedSOItem`))
      (add `/Game/Blueprints/CustomWidgets/FileManager/DuplicateNamesWidget.OnSkipAllItemsEventDispatcher` _returnvalue_2 (`|CreateDelegate` :!event `SkipAllDuplicatedSOItems`))
      (`UserWidget.AddToViewport` _returnvalue_2 0)
      (`KismetArrayLibrary.Array_Clear` _duplicatedsoitems)
      (`KismetArrayLibrary.Array_Add` _duplicatedsoitems (`local.NewActorData`))
      (set `local.isSOValid` false)
      (break)))
  (if (`local.isSOValid`)
    (`self.CreateSynOpticonActorFromStruct` (`local.NewActorData`))))

(fn `GetAllGazeActorNames`
  (returns (GazeActorNames :type "Array of String"))
  (locals (AllNames :type "Array of String"))
  (for _array_element (`SynOpticonState.GetGazeActorList`)
    (bind _asgaze_actor (cast `GazeActor` _array_element))
    (`KismetArrayLibrary.Array_Add` (`local.AllNames`) (`GazeActor.GetName` _asgaze_actor)))
  (return (`local.AllNames`)))

(fn `GetAllSynopticonActorNames`
  (returns (SynOpticonNames :type "Array of String"))
  (locals (SONames :type "Array of String"))
  (for _array_element (`SynOpticonState.GetSynOpticonActorList`)
    (bind _assyn_opticon_actor (cast `SynOpticonActor` _array_element))
    (bind _returnvalue (`SynOpticonActor.GetActorName` _assyn_opticon_actor))
    (`KismetArrayLibrary.Array_Add` (`local.SONames`) _returnvalue))
  (return (`local.SONames`)))

(fn `HandleDuplicateSOActors`
  (params (DuplicatedItems :type "Array of SynOpticonActorStruct Structure"))
  (locals (DuplicatedSOItems :type "Array of SynOpticonActorStruct Structure") (DuplicateWidget :type "/Game/Blueprints/CustomWidgets/FileManager/DuplicateNamesWidget Object Reference") (AllSONames :type "Array of String"))
  (bind _duplicatewidget (`local.DuplicateWidget`))
  (set `local.DuplicatedSOItems` DuplicatedItems)
  (bind _synopticonnames (`self.GetAllSynopticonActorNames`))
  (set `local.AllSONames` _synopticonnames)
  (bind _returnvalue (`|CreateWidget` "/Game/Blueprints/CustomWidgets/FileManager/DuplicateNamesWidget.DuplicateNamesWidget_C"))
  (set `local.DuplicateWidget` _returnvalue)
  (for _array_element (`local.DuplicatedSOItems`)
    (`/Game/Blueprints/CustomWidgets/FileManager/DuplicateNamesWidget.SetUp` (`local.DuplicateWidget`) (`.ActorName` (break `SynOpticonActorStruct` _array_element)) (`local.AllSONames`)))
  (`UserWidget.AddToViewport` _duplicatewidget 0)
  (add `/Game/Blueprints/CustomWidgets/FileManager/DuplicateNamesWidget.OnRenameEventDispatcher` _duplicatewidget (`|CreateDelegate` :!event `RenameDuplicatedSOItem`))
  (add `/Game/Blueprints/CustomWidgets/FileManager/DuplicateNamesWidget.OnReplaceAllItemsEventDispatcher` _duplicatewidget (`|CreateDelegate` :!event `ReplaceAllDuplicatedSOItems`))
  (add `/Game/Blueprints/CustomWidgets/FileManager/DuplicateNamesWidget.OnReplaceItemEventDispatcher` _duplicatewidget (`|CreateDelegate` :!event `ReplaceOneDuplicatedSOItem`))
  (add `/Game/Blueprints/CustomWidgets/FileManager/DuplicateNamesWidget.OnSkipAllItemsEventDispatcher` _duplicatewidget (`|CreateDelegate` :!event `SkipAllDuplicatedSOItems`))
  (add `/Game/Blueprints/CustomWidgets/FileManager/DuplicateNamesWidget.OnSkipItemEventDispatcher` _duplicatewidget (`|CreateDelegate` :!event `SkipOneDuplicatedSOItem`)))

(fn `IsGazeActorNameAvaliable`
  (params (Name :type String))
  (returns (NameUsed :type Boolean))
  (for _array_element (`SynOpticonState.GetGazeActorList`)
    (bind _asgaze_actor (cast `GazeActor` _array_element))
    (if (`KismetStringLibrary.EqualEqual_StrStr` (`GazeActor.GetName` _asgaze_actor) Name)
      (return true)))
  (return false))